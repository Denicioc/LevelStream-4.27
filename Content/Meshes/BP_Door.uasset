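; BP_Door is a sliding door that a player triggers with E while something overlaps its box.
; Box overlap enables input and opens a Gate that passes the key press into the movement logic.
; A short-Delay loop slides the mesh along local X, using a counter and direction flag as travel limits.
; The door pauses at one end, then slides back and stops.
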(event `self.Box.OnComponentBeginOverlap`
  (params (OverlappedComponent :type "PrimitiveComponent Object Reference") (OtherActor :type "Actor Object Reference") (OtherComp :type "PrimitiveComponent Object Reference") (OtherBodyIndex :type Integer) (bFromSweep :type Boolean) (SweepResult :type "HitResult Structure (by ref)"))
  (bind _counter (`self.Counter`))
  (bind _counter_2 (`self.Counter`))
  (bind _counter_3 (`self.Counter`))
  (`self.EnableInput` (`GameplayStatics.GetPlayerController` 0))
  (goto _label :!via `Open`))

(event `Key|E`
  (params (Key :type "Key Structure"))
  (bind _counter (`self.Counter`))
  (bind _counter_2 (`self.Counter`))
  (bind _counter_3 (`self.Counter`))
  (:`Pressed`
    (`/Engine/EditorBlueprintResources/StandardMacros.Gate` true :!label _label
      (:`Exit`
        (if (`self.Opening`) :!label _label_2
          (if (== _counter_3 0.0)
            (set `self.Opening` false)
            (else
              (`SceneComponent.K2_AddLocalTransform` (`self.StaticMesh`) (`KismetMathLibrary.MakeTransform` (`KismetMathLibrary.MakeVector` (select `bool` (`self.Opening`) :`false` -5.0 :`true` 5.0 :!type "Float (single-precision)"))) false false :!label _label_3)
              (if (== _counter 0.0)
                (set `self.Opening` false))
              (if (== _counter 50.0)
                (set `self.Opening` true))
              (`KismetSystemLibrary.Delay` 0.01)
              (if (`self.Opening`)
                (`/Engine/EditorBlueprintResources/StandardMacros.DecrementFloat` _counter_2
                  (:`  `
                    (goto _label_2)))
                (else
                  (`/Engine/EditorBlueprintResources/StandardMacros.IncrementFloat` _counter_2
                    (:`  `
                      (goto _label_2)))))))
          (elif (== _counter_3 50.0)
            (set `self.Opening` true)
            (`KismetSystemLibrary.Delay` 3.0)
            (goto _label_2)
            (else
              (goto _label_3))))))))

(event `self.Box.OnComponentEndOverlap`
  (params (OverlappedComponent :type "PrimitiveComponent Object Reference") (OtherActor :type "Actor Object Reference") (OtherComp :type "PrimitiveComponent Object Reference") (OtherBodyIndex :type Integer))
  (`self.DisableInput` (`GameplayStatics.GetPlayerController` 0))
  (goto _label :!via `Close`))

(fn `UserConstructionScript`)