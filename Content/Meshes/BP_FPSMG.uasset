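; Weapon pickup for the FPS character that grants an SMG, Gatling or gas gun according to its GunSelected enum.
; From BeginPlay, a self-looping short Delay spins the skeletal mesh and bobs it up and down, using a counter to flip direction.
; PickUp copies gun type, fire settings and material to the player, destroys the actor, then calls GetWeapon to set the owned flag and selected slot.
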(event `self.ReceiveBeginPlay`
  (bind _counter (`self.Counter`))
  (bind _counter_2 (`self.Counter`))
  (`SceneComponent.K2_AddLocalTransform` (`self.SkeletalMesh`) (`KismetMathLibrary.MakeTransform` (`KismetMathLibrary.MakeVector` 0.0 0.0 (select `bool` (`self.Floating`) :`false` 0.5 :`true` -0.5 :!type "Float (single-precision)")) (struct :`Yaw` 0.5) (2.0 2.0 2.0)) false false :!label _label)
  (if (== _counter_2 0.0)
    (`|ExecutionSequence`
      (:`then_0`
        (set `self.Floating` false))
      (:`then_1`
        (if (== _counter_2 100.0) :!label _label_2
          (`|ExecutionSequence`
            (:`then_0`
              (set `self.Floating` true))
            (:`then_1`
              (`KismetSystemLibrary.Delay` 0.01 :!label _label_3)
              (if (`self.Floating`)
                (`/Engine/EditorBlueprintResources/StandardMacros.DecrementFloat` _counter
                  (:`  `
                    _))
                (else
                  (`/Engine/EditorBlueprintResources/StandardMacros.IncrementFloat` _counter
                    (:`  `
                      _))))
              (set `self.Counter` _counter)
              (goto _label)))
          (else
            (goto _label_3)))))
    (else
      (goto _label_2))))

(event `self.PickUp`
  (bind _asfirst_person_character (cast `/Game/FirstPersonBP/Blueprints/FirstPersonCharacter` (`GameplayStatics.GetPlayerCharacter` 0)))
  (set `/Game/FirstPersonBP/Blueprints/FirstPersonCharacter.GunSelected` (`self.Gun Selected`) _asfirst_person_character)
  (set `/Game/FirstPersonBP/Blueprints/FirstPersonCharacter.AutoFire` (`self.Auto Fire`) _asfirst_person_character)
  (set `/Game/FirstPersonBP/Blueprints/FirstPersonCharacter.FireRate` (`self.Fire Rate`) _asfirst_person_character)
  (`PrimitiveComponent.SetMaterial` (`/Game/FirstPersonBP/Blueprints/FirstPersonCharacter.FP_Gun` _asfirst_person_character) 0 (`self.Material`))
  (`self.K2_DestroyActor`)
  (`self.GetWeapon`))

(fn `GetWeapon`
  (bind _asfirst_person_character (cast `/Game/FirstPersonBP/Blueprints/FirstPersonCharacter` (`GameplayStatics.GetPlayerCharacter` 0) :!pure true))
  (if (`|EnumEquality` (`self.Gun Selected`) "NewEnumerator0")
    (set `/Game/FirstPersonBP/Blueprints/FirstPersonCharacter.2SMG` true _asfirst_person_character)
    (set `/Game/FirstPersonBP/Blueprints/FirstPersonCharacter.GunSelect` 1 _asfirst_person_character)
    (elif (`|EnumEquality` (`self.Gun Selected`) "NewEnumerator1")
      (set `/Game/FirstPersonBP/Blueprints/FirstPersonCharacter.3Gatling` true _asfirst_person_character)
      (set `/Game/FirstPersonBP/Blueprints/FirstPersonCharacter.GunSelect` 2 _asfirst_person_character)
      (elif (`|EnumEquality` (`self.Gun Selected`) "NewEnumerator2")
        (set `/Game/FirstPersonBP/Blueprints/FirstPersonCharacter.4GasGun` true _asfirst_person_character)
        (set `/Game/FirstPersonBP/Blueprints/FirstPersonCharacter.GunSelect` 3 _asfirst_person_character)))))

(fn `UserConstructionScript`
  (`parent.UserConstructionScript`))